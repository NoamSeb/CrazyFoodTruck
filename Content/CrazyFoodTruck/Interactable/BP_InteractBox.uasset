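; BP_InteractBox is an interactable box in CrazyFoodTruck that can be damaged and repaired.
; BeginPlay hooks up the input-prompt and repair-progress widgets and binds damage and restore events, which toggle IsBroken and drive the repair widget's warning and repair states.
; Tick turns the visible prompt, and the repair widget while broken, toward the camera.
; A separate event recolors the forward camera's outline per player from MPC_Outline.
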(event `self.ReceiveBeginPlay`
  ;[0.1927 0.006022 0 0.5] BEGIN PLAY
  (message `IBoxInteract.SubscribeToBoxInteraction` (`WidgetComponent.GetWidget` (`self.W_PlayerInput`)) self)
  (`RepairProgressBillboard.InitializeWidget` (`self.RepairProgressBillboar`) (`self.RepairWidget`))
  (bind _aswbp_repair_progress (cast `/Game/CrazyFoodTruck/Widget/WBP_RepairProgress` (`WidgetComponent.GetWidget` (`self.RepairWidget`))))
  (set `self.RepairWidgetBP` _aswbp_repair_progress)
  (`self.SetRepairProgress` (`self.RepairProgressBillboar`))
  (add `self.OnDamaged` (delegate `OnDamaged_Event`))
  (add `self.OnRestored` (delegate `OnRestored_Event`)))

(event `OnDamaged_Event`
  ;[0.1927 0.006022 0 0.5] BEGIN PLAY
  (`self.CE_OnDamaged`))

(event `OnRestored_Event`
  ;[0.1927 0.006022 0 0.5] BEGIN PLAY
  (`self.CE_OnRestored`))

(event `self.ReceiveTick`
  (params (DeltaSeconds :type "Float (single-precision)"))
  ;[0.15 0 0 0.5] TICK
  (`|ExecutionSequence`
    (:`then_0`
      (if (`self.GetInputVisibilityState`)
        (`self.CE_UpdateWidgetRotation`)
        (`/Engine/EditorBlueprintResources/StandardMacros.DoOnce` false
          (:`Completed`
            (`/Game/CrazyFoodTruck/Widget/WBP_RepairProgress.CE_ShowBarRepair` (`self.RepairWidgetBP`))))))
    (:`then_1`
      (if (`self.IsBroken`)
        (`self.CE_UpdateRepairWidgetRotaiton`)))))

(event `CE_UpdateWidgetRotation`
  ;[0.15 0 0 0.5] UPDATE WIDGET ROTATION
  (`SceneComponent.K2_SetWorldRotation` (`self.W_PlayerInput`) (`KismetMathLibrary.FindLookAtRotation` (`SceneComponent.K2_GetComponentLocation` (`self.W_PlayerInput`)) (`SceneComponent.K2_GetComponentLocation` (`PlayerCameraManager.TransformComponent` (`GameplayStatics.GetPlayerCameraManager` 0)))) false false))

(event `CE_UpdateRepairWidgetRotaiton`
  ;[0.15 0 0 0.5] UPDATE WIDGET ROTATION
  (`SceneComponent.K2_SetWorldRotation` (`self.RepairWidget`) (`KismetMathLibrary.FindLookAtRotation` (`SceneComponent.K2_GetComponentLocation` (`self.RepairWidget`)) (`SceneComponent.K2_GetComponentLocation` (`PlayerCameraManager.TransformComponent` (`GameplayStatics.GetPlayerCameraManager` 0)))) false false))

(event `CE_OnDamaged`
  (set `self.IsBroken` true)
  (`/Game/CrazyFoodTruck/Widget/WBP_RepairProgress.CE_PlayWarning` (`self.RepairWidgetBP`)))

(event `CE_OnRestored`
  (set `self.IsBroken` false)
  (`/Game/CrazyFoodTruck/Widget/WBP_RepairProgress.CE_Repair` (`self.RepairWidgetBP`)))

(event `self.AddOutlineToForwardCamera`
  (params (PlayerIndex :type Integer))
  (`/Engine/EditorBlueprintResources/StandardMacros.IsValid` (`self.ForwardCam`)
    (:`Is Valid`
      (bind _output_get (set `self.Bit_Name` "OutlineColor_P"))
      (bind _returnvalue (`KismetStringLibrary.Concat_StrStr` _output_get (`KismetStringLibrary.Conv_IntToString` (+ PlayerIndex 1))))
      (`KismetSystemLibrary.PrintString` _returnvalue)
      (bind _returnvalue_2 (`KismetMaterialLibrary.GetVectorParameterValue` "/Game/CrazyFoodTruck/Visuals/VFX/Outline/MPC_Outline.MPC_Outline" (`KismetStringLibrary.Conv_StringToName` _returnvalue)))
      (`self.ChangeCameraOutlineColor` _returnvalue_2))
    (:`Is Not Valid`
      (`KismetSystemLibrary.PrintString` "Camera Invalid"))))

(fn `UserConstructionScript`)