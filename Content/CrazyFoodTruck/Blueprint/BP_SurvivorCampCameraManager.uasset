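; Camera pawn for the survivor camp that the first player controller possesses on BeginPlay, built to orbit its spring arm around the yaw axis.
; A timeline, with play rate set from AnimLenght, adds a yaw lerped between zero and a negative full turn to the arm's world rotation on each update.
; Tick restarts the timeline every frame, and its Finished output also replays it.
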(event `self.ReceiveBeginPlay`
  (`Controller.Possess` (`GameplayStatics.GetPlayerController` 0) self)
  (`TimelineComponent.SetPlayRate` (`self.Timeline`) (/ 1.0 (`self.AnimLenght`))))

(event `self.ReceiveTick`
  (params (DeltaSeconds :type "Float (single-precision)"))
  (bind (_direction _timeline_lenght) (`Timeline|Timeline` :!via `PlayFromStart` :!label _label)
    (:`Update`
      (`SceneComponent.K2_AddWorldRotation` (`self.SpringArm`) (`KismetMathLibrary.MakeRotator` 0.0 0.0 (`KismetMathLibrary.Lerp` 0.0 -360.0 _timeline_lenght)) false false))
    (:`Finished`
      (goto _label :!via `PlayFromStart`))))

(fn `UserConstructionScript`)