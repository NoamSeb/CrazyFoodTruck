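; Food truck pawn for Crazy Food Truck that takes zombie hits, heals, crushes entities at the front and bounces off obstacles.
; Health comes from the GameInstance and drives a diegetic life display, with timed invincibility, camera shake and material tint on damage.
; BeginPlay mounts left and right upgrade modules through ModuleManager with levers, gating movement by game phase.
; Death resets upgrades and opens the lose level, while ChangeMap scores and opens SurvivorCamp.
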(event `self.Coll_Box.OnComponentBeginOverlap`
  (params (OverlappedComponent :type "PrimitiveComponent Object Reference") (OtherActor :type "Actor Object Reference") (OtherComp :type "PrimitiveComponent Object Reference") (OtherBodyIndex :type Integer) (bFromSweep :type Boolean) (SweepResult :type "HitResult Structure (by ref)"))
  ; OVERLAPP
  (if (`KismetSystemLibrary.DoesImplementInterface` OtherActor "/Script/CrazyFoodTruck.IEntity")
    (message `IEntity.InteractWithTruck` OtherActor)
    (if (`self.canTakeDamage`)
      (set `self.canTakeDamage` false)
      (`self.CE_CooldownInvicibility`)
      (bind _returnvalue (message `IEntity.IsAZoombie` OtherActor))
      (if _returnvalue
        (bind _returnvalue_2 (message `IEntity.GetDamage` OtherActor))
        (`self.CE_TakeDamage` _returnvalue_2)
        (`NiagaraFunctionLibrary.SpawnSystemAttached` "/Game/CrazyFoodTruck/Visuals/VFX/NS_HitZombieTruck.NS_HitZombieTruck" (`self.mockupCamion`) "None" (`.ImpactPoint` (`GameplayStatics.BreakHitResult` SweepResult)) (struct) "KeepWorldPosition" true)))))

(event `self.ChangeMap`
  ;[0 0 0 0.5] Begin Change Map
  (set `GameDataSubSystem.CurrentGamePhase` "Amelioration" (subsystem `GameDataSubSystem`))
  (`self.HideWidgetCamera`)
  (bind _ascrazy_food_truck_game_mode (cast `CrazyFoodTruckGameMode` (`GameplayStatics.GetGameMode`)))
  (`GameplayStatics.LoadStreamLevelBySoftObjectPtr` "/Game/CrazyFoodTruck/Levels/SurvivorCamp.SurvivorCamp")
  (add `CrazyFoodTruckGameMode.OnFinalScoreShown` _ascrazy_food_truck_game_mode (delegate `OnFinalScoreShown_Event`))
  (`CrazyFoodTruckGameMode.EvaluateFinalScore` _ascrazy_food_truck_game_mode))

(event `self.ReceiveBeginPlay`
  ;[0.09324 0.15 0 0.5] Begin Play
  (`self.CE_CreateAndSetMaterialInstance`)
  (bind _aslever (cast `Lever` (`ChildActorComponent.ChildActor` (`self.RightLever`))))
  (bind _aslever_2 (cast `Lever` (`ChildActorComponent.ChildActor` (`self.LeftLever`))))
  (`ModuleManager.Initialize` (`self.ModuleManager`) (`self.SC_LeftModule`) (`self.SC_RightModule`) _aslever_2 _aslever)
  (bind _asgame_instance_crazy_food_truck (cast `GameInstanceCrazyFoodTruck` (`GameplayStatics.GetGameInstance`)))
  (bind _output_get (set `self.As Game Instance Crazy Food Truck` _asgame_instance_crazy_food_truck))
  (set `self.TruckLife` (`GameInstanceCrazyFoodTruck.CurrentLifeFoodTruck` _output_get))
  (set `self.TruckMaxLife` (`GameInstanceCrazyFoodTruck.MaxLifeFoodTruck` _output_get))
  (bind _output_get_2 (set `self.NameModule` "Module"))
  (`self.AddModuleToTruck` (`KismetStringLibrary.Concat_StrStr` _output_get_2 (`|GetEnumeratorNameAsString` (`GameInstanceCrazyFoodTruck.ModuleUpgradeLeft` (`self.As Game Instance Crazy Food Truck`)))))
  (bind _output_get_3 (set `self.NameModule` "Module"))
  (`self.AddModuleToTruck` (`KismetStringLibrary.Concat_StrStr` _output_get_3 (`|GetEnumeratorNameAsString` (`GameInstanceCrazyFoodTruck.ModuleUpgradeRight` (`self.As Game Instance Crazy Food Truck`)))) "Right")
  (bind _ashud_upgrade_phase (cast `/Game/CrazyFoodTruck/UI/HUD_UpgradePhase` (`PlayerController.GetHUD` (`GameplayStatics.GetPlayerController` 0))))
  (set `self.As HUD Upgrade Phase` _ashud_upgrade_phase)
  (`KismetSystemLibrary.ExecuteConsoleCommand` "SCALABILITY 2" null)
  (`GameplayStatics.SetGamePaused` false)
  (`WidgetBlueprintLibrary.SetInputMode_GameOnly` (`GameplayStatics.GetPlayerController` 0))
  (bind _asbp_life_diegetic (cast `/Game/CrazyFoodTruck/BP/BP_LifeDiegetic` (`ChildActorComponent.ChildActor` (`self.BP_LifeDiegetic`))))
  (bind _output_get_4 (set `self.LifeDiegetic` _asbp_life_diegetic))
  (`/Game/CrazyFoodTruck/BP/BP_LifeDiegetic.CE_UpdateLifeRender` _output_get_4 (`self.TruckMaxLife`) (`self.TruckLife`))
  (if (`|EnumEquality` (`GameDataSubSystem.CurrentGamePhase` (subsystem `GameDataSubSystem`)) "Route")
    (set `self.MovementEnable` false)
    (`KismetSystemLibrary.Delay` 10.0)
    (set `self.MovementEnable` true)
    (else
      (set `self.MovementEnable` false)))
  (`KismetSystemLibrary.Delay` 1.0)
  (if (`|EnumEquality` (`GameDataSubSystem.CurrentGamePhase` (subsystem `GameDataSubSystem`)) "Route")
    (bind _returnvalue (`|CreateWidget` "/Game/CrazyFoodTruck/UI/WBP/RoadProgress/WBP_RoadProgress.WBP_RoadProgress_C"))
    (`UserWidget.AddToViewport` _returnvalue 0))
  (`GameplayStatics.PlaySound2D` "/Game/CrazyFoodTruck/Sounds/SFX/SFX_Conduite/SFX_Conduite_Idle/SFX_Conduite_IDLE_02.SFX_Conduite_IDLE_02" 1.0 1.0 0.0 null null))

(event `OnFinalScoreShown_Event`
  (bind _as_hud_upgrade_phase (`self.As HUD Upgrade Phase`))
  ;[0 0 0 0.5] Begin Change Map
  (`/Game/CrazyFoodTruck/UI/HUD_UpgradePhase.CE_CreateFade` _as_hud_upgrade_phase)
  (`/Game/CrazyFoodTruck/UI/HUD_UpgradePhase.CE_1to1forScore` _as_hud_upgrade_phase)
  (`KismetSystemLibrary.Delay` 3.25)
  (`GameplayStatics.OpenLevelBySoftObjectPtr` "/Game/CrazyFoodTruck/Levels/SurvivorCamp.SurvivorCamp"))

(event `self.Root.OnComponentHit`
  (params (HitComponent :type "PrimitiveComponent Object Reference") (OtherActor :type "Actor Object Reference") (OtherComp :type "PrimitiveComponent Object Reference") (NormalImpulse :type "Vector Structure") (Hit :type "HitResult Structure (by ref)"))
  (if (not (`self.bShouldBounceBack`))
    (`self.BounceBackOnHit`)
    (`SoundManager.PlaySFX` (`SoundManager.Get`) "ECC_Accident" self)
    (for _index (range (`GameplayStatics.GetNumPlayerControllers`))
      (`PlayerController.K2_ClientPlayForceFeedback` (`GameplayStatics.GetPlayerController` _index) "/Game/CrazyFoodTruck/FF_Tire.FF_Tire" "None" false false false))))

(event `CE_TakeDamage`
  (params (Damage :type Integer))
  (bind _as_game_instance_crazy_food_truck (`self.As Game Instance Crazy Food Truck`))
  ; TAKE DAMAGE
  (bind _output_get (set `GameInstanceCrazyFoodTruck.CurrentLifeFoodTruck` (- (`GameInstanceCrazyFoodTruck.CurrentLifeFoodTruck` _as_game_instance_crazy_food_truck) Damage) _as_game_instance_crazy_food_truck))
  (bind _output_get_2 (set `self.TruckLife` _output_get))
  (`/Game/CrazyFoodTruck/BP/BP_LifeDiegetic.CE_UpdateLifeRender` (`self.LifeDiegetic`) (`self.TruckMaxLife`) _output_get_2)
  (`ShakeController.StartShake` (`self.ShakeController`) "ZombieHit")
  ;; Check Death
  (if (<= _output_get_2 0)
    (`self.CE_Death`)
    (else
      (`SoundManager.PlaySFX` (`SoundManager.Get`) "ECC_ZombieAttack" self)
      (`self.CE_ChangeColorTruck`))))

(event `CE_Heal`
  (params (Heal :type Integer))
  (bind _as_game_instance_crazy_food_truck (`self.As Game Instance Crazy Food Truck`))
  (bind _maxlifefoodtruck (`GameInstanceCrazyFoodTruck.MaxLifeFoodTruck` _as_game_instance_crazy_food_truck))
  (bind _returnvalue (+ Heal (`GameInstanceCrazyFoodTruck.CurrentLifeFoodTruck` _as_game_instance_crazy_food_truck)))
  ; HEAL
  (if (>= _returnvalue _maxlifefoodtruck)
    (bind _output_get (set `GameInstanceCrazyFoodTruck.CurrentLifeFoodTruck` _maxlifefoodtruck _as_game_instance_crazy_food_truck))
    (set `self.TruckLife` _output_get)
    (else
      (bind _output_get_2 (set `GameInstanceCrazyFoodTruck.CurrentLifeFoodTruck` _returnvalue _as_game_instance_crazy_food_truck))
      (set `self.TruckLife` _output_get_2)))
  (`/Game/CrazyFoodTruck/BP/BP_LifeDiegetic.CE_UpdateLifeRender` (`self.LifeDiegetic`) (`self.TruckMaxLife`) (`self.TruckLife`)))

(event `CE_CreateAndSetMaterialInstance`
  ; Set Material and ISntance
  (bind _returnvalue (`PrimitiveComponent.CreateDynamicMaterialInstance` (`self.mockupCamion`) 0 "/Game/CrazyFoodTruck/Assets/Truck/M_Truck.M_Truck" "None"))
  (bind _output_get (set `self.MaterialInstance` _returnvalue))
  (`PrimitiveComponent.SetMaterial` (`self.mockupCamion`) 0 _output_get))

(event `CE_Death`
  (bind _returnvalue (subsystem `FoodTruckDataSubSystem`))
  (bind _as_hud_upgrade_phase (`self.As HUD Upgrade Phase`))
  ; DEATH
  (set `FloatingPawnMovement.Acceleration` 0.0 (`self.FloatingPawnMovement`))
  (set `GameDataSubSystem.LevelNumber` 0 (subsystem `GameDataSubSystem`))
  (set `FoodTruckDataSubSystem.DamagePerBullet` 0 _returnvalue)
  (set `FoodTruckDataSubSystem.Heal` 0.0 _returnvalue)
  (set `FoodTruckDataSubSystem.RepairSpeed` 0 _returnvalue)
  (set `FoodTruckDataSubSystem.RotationSpeed` 0.0 _returnvalue)
  (set `FoodTruckDataSubSystem.Speed` 0.0 _returnvalue)
  (set `FoodTruckDataSubSystem.SpeedRecovery` 0.0 _returnvalue)
  (set `FoodTruckDataSubSystem.TruckRotationSpeed` 0.0 _returnvalue)
  (set `FoodTruckDataSubSystem.TurretFireRate` 0.0 _returnvalue)
  (set `FoodTruckDataSubSystem.TurretMaxAmmo` 0 _returnvalue)
  (set `FoodTruckDataSubSystem.TurretRangeDepth` 0.0 _returnvalue)
  (set `FoodTruckDataSubSystem.TurretRangeSide` 0.0 _returnvalue)
  (set `FoodTruckDataSubSystem.TypeBullet` "BulletNormal" _returnvalue)
  (set `GameDataSubSystem.CurrentGamePhase` "Loose" (subsystem `GameDataSubSystem`))
  (`GameplayStatics.LoadStreamLevelBySoftObjectPtr` "/Game/CrazyFoodTruck/Levels/LooseLevel.LooseLevel")
  (`/Game/CrazyFoodTruck/UI/HUD_UpgradePhase.CE_CreateFade` _as_hud_upgrade_phase)
  (`/Game/CrazyFoodTruck/UI/HUD_UpgradePhase.CE_Fade1to0SansLogo` _as_hud_upgrade_phase)
  (`GameplayStatics.OpenLevelBySoftObjectPtr` "/Game/CrazyFoodTruck/Levels/LooseLevel.LooseLevel"))

(event `CE_CooldownInvicibility`
  ; COOLDOWN
  (`KismetSystemLibrary.Delay` (`self.Invicibility Time`))
  (set `self.canTakeDamage` true))

(event `CE_ChangeColorTruck`
  (bind (_direction _alpha) (`Timeline|Color Truck` :!via `PlayFromStart`)
    (:`Update`
      (`MaterialInstanceDynamic.SetScalarParameterValue` (`self.MaterialInstance`) "Color" (`KismetMathLibrary.Lerp` 0.0 0.035 _alpha)))))

(event `self.Coll_ForwardCollision.OnComponentBeginOverlap`
  (params (OverlappedComponent :type "PrimitiveComponent Object Reference") (OtherActor :type "Actor Object Reference") (OtherComp :type "PrimitiveComponent Object Reference") (OtherBodyIndex :type Integer) (bFromSweep :type Boolean) (SweepResult :type "HitResult Structure (by ref)"))
  ; OVERLAPP FRONT
  (if (`KismetSystemLibrary.DoesImplementInterface` OtherActor "/Script/CrazyFoodTruck.IEntity")
    (message `IEntity.CrushUnderTruckBlueprint` OtherActor 0)))

(event `self.ReceiveUnpossessed`
  (params (OldController :type "Controller Object Reference"))
  (`self.UpdateScreenOutline`)
  (`self.SetTruckState` "Idle"))

(fn `AddModuleToTruck`
  (params (ID :type String) (Side :type "EModuleSide Enum" :default "Left"))
  (bind _leftmodulebox (`self.LeftModuleBox`))
  (bind _rightmodulebox (`self.RightModuleBox`))
  (bind _returnvalue (`ModuleManager.AddModule` (`self.ModuleManager`) ID Side))
  (switch `EModuleSide` Side
    (:`Left`
      (`/Engine/EditorBlueprintResources/StandardMacros.IsValid` (`self.LeftModule`)
        (:`Is Valid`
          (`self.DestroyModuleTruck` "Left"))
        (:`Is Not Valid`
          _))
      ; Left
      (`/Engine/EditorBlueprintResources/StandardMacros.IsValid` (`self.LeftModuleBox`)
        (:`Is Valid`
          (`/Engine/EditorBlueprintResources/StandardMacros.IsValid` (`InteractBox.GetInteractableObject` _leftmodulebox)
            (:`Is Not Valid`
              (`InteractBox.SetInteractableObject` _leftmodulebox _returnvalue)
              (set `self.LeftModule` _returnvalue))))))
    (:`Right`
      (`/Engine/EditorBlueprintResources/StandardMacros.IsValid` (`self.RightModule`)
        (:`Is Valid`
          (`self.DestroyModuleTruck` "Left"))
        (:`Is Not Valid`
          _))
      ; Right
      (`/Engine/EditorBlueprintResources/StandardMacros.IsValid` (`self.RightModuleBox`)
        (:`Is Valid`
          (`/Engine/EditorBlueprintResources/StandardMacros.IsValid` (`InteractBox.GetInteractableObject` _rightmodulebox)
            (:`Is Not Valid`
              (`InteractBox.SetInteractableObject` _rightmodulebox _returnvalue)
              (set `self.RightModule` _returnvalue))))))))

(fn `DestroyModuleTruck`
  (params (Side :type "EModuleSide Enum" :default "Left"))
  (bind _rightmodule (`self.RightModule`))
  (bind _leftmodule (`self.LeftModule`))
  (switch `EModuleSide` Side
    (:`Left`
      (`/Engine/EditorBlueprintResources/StandardMacros.IsValid` _leftmodule
        (:`Is Valid`
          (`self.K2_DestroyActor` _leftmodule))))
    (:`Right`
      (`/Engine/EditorBlueprintResources/StandardMacros.IsValid` _rightmodule
        (:`Is Valid`
          (`self.K2_DestroyActor` _rightmodule))))))

(fn `UserConstructionScript`)