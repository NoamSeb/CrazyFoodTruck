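; Player food truck pawn that takes zombie hits, crushes entities in its path and carries upgrade modules.
; On BeginPlay it fills its life and mounts left and right modules through ModuleManager, using IDs built from GameInstance upgrade enums.
; Zombie overlaps deal damage behind an invincibility cooldown, updating a diegetic life display; death shows the menu and resets upgrades.
; It also handles healing via GameInstance life and travel to the SurvivorCamp upgrade phase.
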(event `self.ReceiveBeginPlay`
  ;[0.09324 0.15 0 0.5] Begin Play
  (bind _asgame_instance_crazy_food_truck (cast `GameInstanceCrazyFoodTruck` (`GameplayStatics.GetGameInstance`)))
  (set `self.As Game Instance Crazy Food Truck` _asgame_instance_crazy_food_truck)
  (`WidgetBlueprintLibrary.SetInputMode_GameOnly` (`GameplayStatics.GetPlayerController` 0))
  (set `self.TruckLife` (`self.TruckMaxLife`))
  (bind _asbp_life_diegetic (cast `/Game/CrazyFoodTruck/BP/BP_LifeDiegetic` (`ChildActorComponent.ChildActor` (`self.BP_LifeDiegetic`))))
  (set `self.LifeDiegetic` _asbp_life_diegetic)
  (`ModuleManager.Initialize` (`self.ModuleManager`) (`self.SC_LeftModule`) (`self.SC_RightModule`))
  (`KismetSystemLibrary.Delay` 1.0)
  (bind _output_get (set `self.NameModule` "Module"))
  (`self.AddModuleToTruck` (`KismetStringLibrary.Concat_StrStr` _output_get (`|GetEnumeratorNameAsString` (`GameInstanceCrazyFoodTruck.ModuleUpgradeLeft` (`self.As Game Instance Crazy Food Truck`)))))
  (bind _output_get_2 (set `self.NameModule` "Module"))
  (`self.AddModuleToTruck` (`KismetStringLibrary.Concat_StrStr` _output_get_2 (`|GetEnumeratorNameAsString` (`GameInstanceCrazyFoodTruck.ModuleUpgradeRight` (`self.As Game Instance Crazy Food Truck`)))) "Right"))

(event `self.Coll_Box.OnComponentBeginOverlap`
  (params (OverlappedComponent :type "PrimitiveComponent Object Reference") (OtherActor :type "Actor Object Reference") (OtherComp :type "PrimitiveComponent Object Reference") (OtherBodyIndex :type Integer) (bFromSweep :type Boolean) (SweepResult :type "HitResult Structure (by ref)"))
  ; OVERLAPP
  (if (`KismetSystemLibrary.DoesImplementInterface` OtherActor "/Script/CrazyFoodTruck.IEntity")
    (message `IEntity.InteractWithTruck` OtherActor)
    (if (`self.canTakeDamage`)
      (set `self.canTakeDamage` false)
      (`self.CE_CooldownInvicibility`)
      (bind _returnvalue (message `IEntity.IsAZoombie` OtherActor))
      (if _returnvalue
        (bind _returnvalue_2 (message `IEntity.GetDamage` OtherActor))
        (`self.CE_TakeDamage` _returnvalue_2)
        (`NiagaraFunctionLibrary.SpawnSystemAtLocation` "/Game/CrazyFoodTruck/Visuals/VFX/NS_HitZombieTruck.NS_HitZombieTruck" (`.ImpactPoint` (`GameplayStatics.BreakHitResult` SweepResult)))))))

(event `self.ChangeMap`
  ;[0 0 0 0.5] Change Map
  (bind _returnvalue (`GameplayStatics.SpawnSoundAttached` "/Game/CrazyFoodTruck/Sounds/MS_SFX.MS_SFX" (`self.mockupCamion`) "None" (0.0 0.0 0.0) (struct) "KeepRelativeOffset" false 1.0 1.0 0.0 null null))
  (`AudioParameterControllerInterface.SetIntParameter` _returnvalue "soundIndex" 0)
  (`AudioComponent.Play` _returnvalue 0.0)
  (bind _boutsuccess (`LevelStreamingDynamic.LoadLevelInstanceBySoftObjectPtr` "/Game/CrazyFoodTruck/Levels/SurvivorCamp.SurvivorCamp" (0.0 0.0 0.0) (struct) "" null))
  (if _boutsuccess
    (set `GameDataSubSystem.CurrentGamePhase` "Amelioration" (subsystem `GameDataSubSystem`))
    (`GameplayStatics.OpenLevelBySoftObjectPtr` "/Game/CrazyFoodTruck/Levels/SurvivorCamp.SurvivorCamp")))

(event `CE_TakeDamage`
  (params (Damage :type Integer))
  ; TAKE DAMAGE
  (bind _output_get (set `self.TruckLife` (- (`self.TruckLife`) Damage)))
  (`/Game/CrazyFoodTruck/BP/BP_LifeDiegetic.CE_UpdateLifeRender` (`self.LifeDiegetic`) (`self.TruckMaxLife`) _output_get)
  (`ShakeController.StartShake` (`self.ShakeController`) "ZombieHit")
  ;; Check Death
  (if (<= _output_get 0)
    (`self.CE_Death`)))

(event `CE_Death`
  (bind _returnvalue (`GameplayStatics.GetPlayerController` 0))
  (bind _returnvalue_2 (subsystem `FoodTruckDataSubSystem`))
  ; DEATH
  (set `FloatingPawnMovement.Acceleration` 0.0 (`self.FloatingPawnMovement`))
  (`WidgetBlueprintLibrary.SetInputMode_UIOnlyEx` _returnvalue null)
  (bind _returnvalue_3 (`|CreateWidget` "/Game/CrazyFoodTruck/UI/WBP/Menus/WBP_Menu.WBP_Menu_C" _returnvalue))
  (`UserWidget.AddToViewport` _returnvalue_3 0)
  (set `GameDataSubSystem.LevelNumber` 0 (subsystem `GameDataSubSystem`))
  (set `FoodTruckDataSubSystem.DamagePerBullet` 0 _returnvalue_2)
  (set `FoodTruckDataSubSystem.Heal` 0.0 _returnvalue_2)
  (set `FoodTruckDataSubSystem.RepairSpeed` 0.0 _returnvalue_2)
  (set `FoodTruckDataSubSystem.RotationSpeed` 0.0 _returnvalue_2)
  (set `FoodTruckDataSubSystem.Speed` 0.0 _returnvalue_2)
  (set `FoodTruckDataSubSystem.SpeedRecovery` 0.0 _returnvalue_2)
  (set `FoodTruckDataSubSystem.TruckRotationSpeed` 0.0 _returnvalue_2)
  (set `FoodTruckDataSubSystem.TurretFireRate` 0.0 _returnvalue_2)
  (set `FoodTruckDataSubSystem.TurretMaxAmmo` 0 _returnvalue_2)
  (set `FoodTruckDataSubSystem.TurretRangeDepth` 0.0 _returnvalue_2)
  (set `FoodTruckDataSubSystem.TurretRangeSide` 0.0 _returnvalue_2)
  (set `FoodTruckDataSubSystem.TypeBullet` "BulletNormal" _returnvalue_2))

(event `CE_CooldownInvicibility`
  ; COOLDOWN
  (`KismetSystemLibrary.Delay` (`self.Invicibility Time`))
  (set `self.canTakeDamage` true))

(event `self.Coll_ForwardCollision.OnComponentBeginOverlap`
  (params (OverlappedComponent :type "PrimitiveComponent Object Reference") (OtherActor :type "Actor Object Reference") (OtherComp :type "PrimitiveComponent Object Reference") (OtherBodyIndex :type Integer) (bFromSweep :type Boolean) (SweepResult :type "HitResult Structure (by ref)"))
  ; Crush Under Truck
  (if (`KismetSystemLibrary.DoesImplementInterface` OtherActor "/Script/CrazyFoodTruck.IEntity")
    (message `IEntity.CrushUnderTruckBlueprint` OtherActor 0)))

(event `CE_Heal`
  (params (Heal :type Integer))
  (bind _as_game_instance_crazy_food_truck (`self.As Game Instance Crazy Food Truck`))
  (bind _maxlifefoodtruck (`GameInstanceCrazyFoodTruck.MaxLifeFoodTruck` _as_game_instance_crazy_food_truck))
  (bind _returnvalue (+ Heal (`GameInstanceCrazyFoodTruck.CurrentLifeFoodTruck` _as_game_instance_crazy_food_truck)))
  ; HEAL
  (if (>= _returnvalue _maxlifefoodtruck)
    (bind _output_get (set `GameInstanceCrazyFoodTruck.CurrentLifeFoodTruck` _maxlifefoodtruck _as_game_instance_crazy_food_truck))
    (set `self.TruckLife` _output_get)
    (else
      (bind _output_get_2 (set `GameInstanceCrazyFoodTruck.CurrentLifeFoodTruck` _returnvalue _as_game_instance_crazy_food_truck))
      (set `self.TruckLife` _output_get_2)))
  (`/Game/CrazyFoodTruck/BP/BP_LifeDiegetic.CE_UpdateLifeRender` (`self.LifeDiegetic`) (`self.TruckMaxLife`) (`self.TruckLife`)))

(event `self.ReceiveUnpossessed`
  (params (OldController :type "Controller Object Reference"))
  (`self.UpdateScreenOutline`)
  (set `self.TruckState` "Idle"))

(fn `AddModuleToTruck`
  (params (ID :type String) (Side :type "EModuleSide Enum" :default "Left"))
  (bind _leftmodulebox (`self.LeftModuleBox`))
  (bind _rightmodulebox (`self.RightModuleBox`))
  (bind _returnvalue (`ModuleManager.AddModule` (`self.ModuleManager`) ID Side))
  (switch `EModuleSide` Side
    (:`Left`
      (`/Engine/EditorBlueprintResources/StandardMacros.IsValid` (`self.LeftModule`)
        (:`Is Valid`
          (`self.DestroyModuleTruck` "Left"))
        (:`Is Not Valid`
          _))
      ; Left
      (`/Engine/EditorBlueprintResources/StandardMacros.IsValid` (`self.LeftModuleBox`)
        (:`Is Valid`
          (`/Engine/EditorBlueprintResources/StandardMacros.IsValid` (`InteractBox.GetInteractableObject` _leftmodulebox)
            (:`Is Not Valid`
              (`InteractBox.SetInteractableObject` _leftmodulebox _returnvalue)
              (set `self.LeftModule` _returnvalue))))))
    (:`Right`
      (`/Engine/EditorBlueprintResources/StandardMacros.IsValid` (`self.RightModule`)
        (:`Is Valid`
          (`self.DestroyModuleTruck` "Left"))
        (:`Is Not Valid`
          _))
      ; Right
      (`/Engine/EditorBlueprintResources/StandardMacros.IsValid` (`self.RightModuleBox`)
        (:`Is Valid`
          (`/Engine/EditorBlueprintResources/StandardMacros.IsValid` (`InteractBox.GetInteractableObject` _rightmodulebox)
            (:`Is Not Valid`
              (`InteractBox.SetInteractableObject` _rightmodulebox _returnvalue)
              (set `self.RightModule` _returnvalue))))))))

(fn `DestroyModuleTruck`
  (params (Side :type "EModuleSide Enum" :default "Left"))
  (bind _rightmodule (`self.RightModule`))
  (bind _leftmodule (`self.LeftModule`))
  (switch `EModuleSide` Side
    (:`Left`
      (`/Engine/EditorBlueprintResources/StandardMacros.IsValid` _leftmodule
        (:`Is Valid`
          (`self.K2_DestroyActor` _leftmodule))))
    (:`Right`
      (`/Engine/EditorBlueprintResources/StandardMacros.IsValid` _rightmodule
        (:`Is Valid`
          (`self.K2_DestroyActor` _rightmodule))))))

(fn `UserConstructionScript`)