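; BP_TestPlayer is a test player Blueprint that marks its Cube for a per-player outline using custom depth.
; On BeginPlay or possession, it reads a Bit_P scalar from MPC_Outline, numbered by ArrayIndex plus one, and applies it as the stencil value.
; Unpossession or a negative index turns custom depth off.
; The controller-array lookup that would set ArrayIndex is unconnected and never runs.
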(event `self.ReceiveBeginPlay`
  (bind _cube (`self.Cube`))
  (if (>= (`self.Array Index`) 0) :!label _label
    (bind _output_get (set `self.Bit_Name` "Bit_P"))
    (bind _returnvalue (`KismetMaterialLibrary.GetScalarParameterValue` "/Game/CrazyFoodTruck/Visuals/VFX/Outline/MPC_Outline.MPC_Outline" (`KismetStringLibrary.Conv_StringToName` (`KismetStringLibrary.Concat_StrStr` _output_get (`KismetStringLibrary.Conv_IntToString` (+ (`self.Array Index`) 1))))))
    (`PrimitiveComponent.SetCustomDepthStencilValue` _cube (`KismetMathLibrary.FTrunc` _returnvalue))
    (`PrimitiveComponent.SetRenderCustomDepth` _cube true)
    (else
      (`KismetSystemLibrary.PrintString` "Index not found" true true (struct :`R` 1.0 :`A` 1.0))
      (`PrimitiveComponent.SetRenderCustomDepth` (`self.Cube`) false :!label _label_2))))

(event `self.ReceivePossessed`
  (params (NewController :type "Controller Object Reference"))
  (goto _label))

(event `self.ReceiveUnpossessed`
  (params (OldController :type "Controller Object Reference"))
  (goto _label_2))

(fn `UserConstructionScript`)