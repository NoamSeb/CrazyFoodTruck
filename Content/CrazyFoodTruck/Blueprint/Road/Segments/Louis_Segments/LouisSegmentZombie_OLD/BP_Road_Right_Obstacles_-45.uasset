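; Road segment actor for Crazy Food Truck, built procedurally along a spline at construction time.
; The construction script lays brick spline meshes along MainRoad and moves EndRoadPoint to the spline's last point.
; It rebuilds left and right blocker splines by offsetting each road point along local Y, then spawns colliding spline meshes on them as side barriers.
; The event graph is empty, so all logic lives in construction.
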(fn `SpawnBlockerOnSpline`
  (bind _leftblocker (`self.LeftBlocker`))
  (bind _rightblocker (`self.RightBlocker`))
  (`|ExecutionSequence`
    (:`then_0`
      (for _index (range (+ (- (`SplineComponent.GetNumberOfSplinePoints` (`self.LeftBlocker`)) 2) 1))
        (bind _returnvalue (`AddComponent|NODE_AddSplineMeshComponent-3`))
        (`SplineMeshComponent.SetForwardAxis` _returnvalue "X" true)
        (`PrimitiveComponent.SetMaterial` _returnvalue 0 "/Game/StarterContent/Materials/M_Basic_Floor.M_Basic_Floor")
        (bind _returnvalue_2 (+ _index 1))
        (`SplineMeshComponent.SetStartAndEnd` _returnvalue (`SplineComponent.GetLocationAtSplinePoint` _leftblocker _index "Local") (`SplineComponent.GetTangentAtSplinePoint` _leftblocker _index "Local") (`SplineComponent.GetLocationAtSplinePoint` _leftblocker _returnvalue_2 "Local") (`SplineComponent.GetTangentAtSplinePoint` _leftblocker _returnvalue_2 "Local") true)
        (`PrimitiveComponent.SetCollisionEnabled` _returnvalue "QueryAndPhysics")
        (`PrimitiveComponent.SetCollisionObjectType` _returnvalue "ECC_GameTraceChannel1")
        (`SceneComponent.K2_AttachToComponent` _returnvalue (`self.LeftBlocker`) "None" "KeepRelative" "KeepRelative" "KeepRelative" true)))
    (:`then_1`
      (for _index_2 (range (+ (- (`SplineComponent.GetNumberOfSplinePoints` (`self.RightBlocker`)) 2) 1))
        (bind _returnvalue_3 (`AddComponent|NODE_AddSplineMeshComponent-4`))
        (`SplineMeshComponent.SetForwardAxis` _returnvalue_3 "X" true)
        (`PrimitiveComponent.SetMaterial` _returnvalue_3 0 "/Game/StarterContent/Materials/M_Basic_Floor.M_Basic_Floor")
        (bind _returnvalue_4 (+ _index_2 1))
        (`SplineMeshComponent.SetStartAndEnd` _returnvalue_3 (`SplineComponent.GetLocationAtSplinePoint` _rightblocker _index_2 "Local") (`SplineComponent.GetTangentAtSplinePoint` _rightblocker _index_2 "Local") (`SplineComponent.GetLocationAtSplinePoint` _rightblocker _returnvalue_4 "Local") (`SplineComponent.GetTangentAtSplinePoint` _rightblocker _returnvalue_4 "Local") true)
        (`PrimitiveComponent.SetCollisionEnabled` _returnvalue_3 "QueryAndPhysics")
        (`PrimitiveComponent.SetCollisionObjectType` _returnvalue_3 "ECC_GameTraceChannel1")
        (`SceneComponent.K2_AttachToComponent` _returnvalue_3 (`self.RightBlocker`) "None" "KeepRelative" "KeepRelative" "KeepRelative" true)))))

(fn `SyncBlockerToMainRoad`
  (`SplineComponent.ClearSplinePoints` (`self.LeftBlocker`) true)
  (`SplineComponent.ClearSplinePoints` (`self.RightBlocker`) true)
  (for _index (range (`SplineComponent.GetNumberOfSplinePoints` (`self.MainRoad`)))
    (bind (_returnvalue_x _returnvalue_y _returnvalue_z) (`KismetMathLibrary.BreakVector` (`SplineComponent.GetLocationAtSplinePoint` (`self.MainRoad`) _index "Local")))
    (`SplineComponent.AddSplinePoint` (`self.LeftBlocker`) (`KismetMathLibrary.MakeVector` _returnvalue_x (- _returnvalue_y (`self.Offset`)) _returnvalue_z) "Local" true)
    (bind (_returnvalue_x_2 _returnvalue_y_2 _returnvalue_z_2) (`KismetMathLibrary.BreakVector` (`SplineComponent.GetLocationAtSplinePoint` (`self.MainRoad`) _index "Local")))
    (`SplineComponent.AddSplinePoint` (`self.RightBlocker`) (`KismetMathLibrary.MakeVector` _returnvalue_x_2 (+ _returnvalue_y_2 (`self.Offset`)) _returnvalue_z_2) "Local" true)))

(fn `UserConstructionScript`
  (bind _mainroad (`self.MainRoad`))
  (bind _mainroad_2 (`self.MainRoad`))
  (`SplineComponent.SetLocationAtSplinePoint` (`self.MainRoad`) 0 (`SceneComponent.RelativeLocation` (`self.StartRoadPoint`)) "Local" true)
  (`SceneComponent.K2_SetWorldLocation` (`self.EndRoadPoint`) (`SplineComponent.GetLocationAtSplinePoint` _mainroad_2 (- (`SplineComponent.GetNumberOfSplinePoints` _mainroad_2) 1) "Local") false false)
  (for _index (range (+ (- (`SplineComponent.GetNumberOfSplinePoints` (`self.MainRoad`)) 2) 1))
    (bind _returnvalue (`AddComponent|NODE_AddSplineMeshComponent-2`))
    (`SplineMeshComponent.SetForwardAxis` _returnvalue "X" true)
    (`PrimitiveComponent.SetMaterial` _returnvalue 0 "/Game/StarterContent/Materials/M_Brick_Clay_New.M_Brick_Clay_New")
    (bind _returnvalue_2 (+ _index 1))
    (bind _returnvalue_3 (`SplineComponent.GetLocationAtSplinePoint` _mainroad _returnvalue_2 "Local"))
    (`SplineMeshComponent.SetStartAndEnd` _returnvalue (`SplineComponent.GetLocationAtSplinePoint` _mainroad _index "Local") (`SplineComponent.GetTangentAtSplinePoint` _mainroad _index "Local") _returnvalue_3 (`SplineComponent.GetTangentAtSplinePoint` _mainroad _returnvalue_2 "Local") true)
    (`SceneComponent.K2_AttachToComponent` _returnvalue (`self.MainRoad`) "None" "KeepRelative" "KeepRelative" "KeepRelative" true))
  (`self.SyncBlockerToMainRoad`)
  (`self.SpawnBlockerOnSpline`)
  ; Set End Point location at the end of the spline
  (`SceneComponent.K2_SetWorldLocation` (`self.EndRoadPoint`) _returnvalue_3 false false))