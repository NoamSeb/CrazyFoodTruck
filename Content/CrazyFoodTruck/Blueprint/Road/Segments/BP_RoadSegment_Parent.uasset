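; Parent road segment Blueprint that builds a spline road with side blockers and wires up its zombie spawn waves.
; The construction script lays spline meshes along MainRoad, moves EndRoadPoint to its end, and builds colliding blockers from custom splines or world-Y offset copies of the road.
; BeginPlay gathers child spawn areas and the zombie trigger, assigns each wave the area matching its target point, then debug-prints wave validity.
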(event `self.ReceiveBeginPlay`
  (bind _triggerzombie (`self.triggerZombie`))
  (for _array_element (`self.GetAllChildActors` true)
    (bind _asarea_zombie_spawn (cast `AreaZombieSpawn` _array_element)
      (:`then`
        (`KismetArrayLibrary.Array_AddUnique` (`self.ListArea`) _asarea_zombie_spawn))
      (:`CastFailed`
        (bind _astrigger_zombie (cast `TriggerZombie` _array_element))
        (set `self.triggerZombie` _astrigger_zombie))))
  (`/Engine/EditorBlueprintResources/StandardMacros.IsValid` _triggerzombie
    (:`Is Valid`
      (for (_array_element_2 _array_index) (`TriggerZombie.SpawnWaves` _triggerzombie)
        (for _array_element_3 (`self.ListArea`)
          (if (== (`KismetMathLibrary.Conv_ByteToInt` (`AreaZombieSpawn.PositionSpawn` _array_element_3)) (`KismetMathLibrary.Conv_ByteToInt` (`.TargetZombiePoint` (break `WaveStructure` _array_element_2))))
            (setmembers `WaveStructure` :`StructRef` (`|GetArrayItem` (`TriggerZombie.SpawnWaves` (`self.triggerZombie`)) _array_index) :`ZoneSpawn` _array_element_3))))
      (`self.CE_CheckCompleted`))))

(event `CE_CheckCompleted`
  (for _array_element (`TriggerZombie.SpawnWaves` (`self.triggerZombie`))
    (`/Engine/EditorBlueprintResources/StandardMacros.IsValid` (`.ZoneSpawn` (break `WaveStructure` _array_element))
      (:`Is Valid`
        (`KismetSystemLibrary.PrintString` "VALID"))
      (:`Is Not Valid`
        (`KismetSystemLibrary.PrintString` "NOT VALID")))))

(fn `SpawnBlockerOnCustomSplines`
  (bind _customrightblockerspline (`self.CustomRightBlockerSpline`))
  (bind _customleftblockerspline (`self.CustomLeftBlockerSpline`))
  (`|ExecutionSequence`
    (:`then_0`
      (for _index (range (+ (- (`SplineComponent.GetNumberOfSplinePoints` (`self.CustomLeftBlockerSpline`)) 2) 1))
        (bind _returnvalue (`AddComponent|NODE_AddSplineMeshComponent-5`))
        (`SplineMeshComponent.SetForwardAxis` _returnvalue "X" true)
        (`PrimitiveComponent.SetMaterial` _returnvalue 0 "/InterchangeAssets/gltf/MaterialInstances/MI_Default_Opaque.MI_Default_Opaque")
        (bind _returnvalue_2 (+ _index 1))
        (`SplineMeshComponent.SetStartAndEnd` _returnvalue (`SplineComponent.GetLocationAtSplinePoint` _customleftblockerspline _index "Local") (`SplineComponent.GetTangentAtSplinePoint` _customleftblockerspline _index "Local") (`SplineComponent.GetLocationAtSplinePoint` _customleftblockerspline _returnvalue_2 "Local") (`SplineComponent.GetTangentAtSplinePoint` _customleftblockerspline _returnvalue_2 "Local") true)
        (`PrimitiveComponent.SetCollisionEnabled` _returnvalue "QueryAndPhysics")
        (`PrimitiveComponent.SetCollisionObjectType` _returnvalue "ECC_GameTraceChannel1")
        (`SceneComponent.K2_AttachToComponent` _returnvalue (`self.CustomLeftBlockerSpline`) "None" "KeepRelative" "KeepRelative" "KeepRelative" true)))
    (:`then_1`
      (for _index_2 (range (+ (- (`SplineComponent.GetNumberOfSplinePoints` (`self.CustomRightBlockerSpline`)) 2) 1))
        (bind _returnvalue_3 (`AddComponent|NODE_AddSplineMeshComponent-6`))
        (`SplineMeshComponent.SetForwardAxis` _returnvalue_3 "X" true)
        (`PrimitiveComponent.SetMaterial` _returnvalue_3 0 "/InterchangeAssets/gltf/MaterialInstances/MI_Default_Opaque.MI_Default_Opaque")
        (bind _returnvalue_4 (+ _index_2 1))
        (`SplineMeshComponent.SetStartAndEnd` _returnvalue_3 (`SplineComponent.GetLocationAtSplinePoint` _customrightblockerspline _index_2 "Local") (`SplineComponent.GetTangentAtSplinePoint` _customrightblockerspline _index_2 "Local") (`SplineComponent.GetLocationAtSplinePoint` _customrightblockerspline _returnvalue_4 "Local") (`SplineComponent.GetTangentAtSplinePoint` _customrightblockerspline _returnvalue_4 "Local") true)
        (`PrimitiveComponent.SetCollisionEnabled` _returnvalue_3 "QueryAndPhysics")
        (`PrimitiveComponent.SetCollisionObjectType` _returnvalue_3 "ECC_GameTraceChannel1")
        (`SceneComponent.K2_AttachToComponent` _returnvalue_3 (`self.CustomRightBlockerSpline`) "None" "KeepRelative" "KeepRelative" "KeepRelative" true)))))

(fn `SpawnBlockerOnSpline`
  (bind _leftblocker (`self.LeftBlocker`))
  (bind _rightblocker (`self.RightBlocker`))
  (`|ExecutionSequence`
    (:`then_0`
      (for _index (range (+ (- (`SplineComponent.GetNumberOfSplinePoints` (`self.LeftBlocker`)) 2) 1))
        (bind _returnvalue (`AddComponent|NODE_AddSplineMeshComponent-3`))
        (`SplineMeshComponent.SetForwardAxis` _returnvalue "X" true)
        (`PrimitiveComponent.SetMaterial` _returnvalue 0 "/Game/StarterContent/Materials/M_Basic_Floor.M_Basic_Floor")
        (bind _returnvalue_2 (+ _index 1))
        (`SplineMeshComponent.SetStartAndEnd` _returnvalue (`SplineComponent.GetLocationAtSplinePoint` _leftblocker _index "World") (`SplineComponent.GetTangentAtSplinePoint` _leftblocker _index "World") (`SplineComponent.GetLocationAtSplinePoint` _leftblocker _returnvalue_2 "World") (`SplineComponent.GetTangentAtSplinePoint` _leftblocker _returnvalue_2 "World") true)
        (`PrimitiveComponent.SetCollisionEnabled` _returnvalue "QueryAndPhysics")
        (`PrimitiveComponent.SetCollisionObjectType` _returnvalue "ECC_GameTraceChannel1")
        (`SceneComponent.K2_AttachToComponent` _returnvalue (`self.LeftBlocker`) "None" "KeepRelative" "KeepRelative" "KeepRelative" true)))
    (:`then_1`
      (for _index_2 (range (+ (- (`SplineComponent.GetNumberOfSplinePoints` (`self.RightBlocker`)) 2) 1))
        (bind _returnvalue_3 (`AddComponent|NODE_AddSplineMeshComponent-4`))
        (`SplineMeshComponent.SetForwardAxis` _returnvalue_3 "X" true)
        (`PrimitiveComponent.SetMaterial` _returnvalue_3 0 "/Game/StarterContent/Materials/M_Basic_Floor.M_Basic_Floor")
        (bind _returnvalue_4 (+ _index_2 1))
        (`SplineMeshComponent.SetStartAndEnd` _returnvalue_3 (`SplineComponent.GetLocationAtSplinePoint` _rightblocker _index_2 "World") (`SplineComponent.GetTangentAtSplinePoint` _rightblocker _index_2 "World") (`SplineComponent.GetLocationAtSplinePoint` _rightblocker _returnvalue_4 "World") (`SplineComponent.GetTangentAtSplinePoint` _rightblocker _returnvalue_4 "World") true)
        (`PrimitiveComponent.SetCollisionEnabled` _returnvalue_3 "QueryAndPhysics")
        (`PrimitiveComponent.SetCollisionObjectType` _returnvalue_3 "ECC_GameTraceChannel1")
        (`SceneComponent.K2_AttachToComponent` _returnvalue_3 (`self.RightBlocker`) "None" "KeepRelative" "KeepRelative" "KeepRelative" true)))))

(fn `SyncBlockerToMainRoad`
  (bind _leftblocker (`self.LeftBlocker`))
  (bind _mainroad (`self.MainRoad`))
  (bind _rightblocker (`self.RightBlocker`))
  (`SplineComponent.ClearSplinePoints` (`self.LeftBlocker`) true)
  (`SplineComponent.ClearSplinePoints` (`self.RightBlocker`) true)
  (for _index (range (`SplineComponent.GetNumberOfSplinePoints` (`self.MainRoad`)))
    (bind (_returnvalue_x _returnvalue_y _returnvalue_z) (`KismetMathLibrary.BreakVector` (`SplineComponent.GetLocationAtSplinePoint` _mainroad _index "World")))
    (`SplineComponent.AddSplinePoint` _leftblocker (`KismetMathLibrary.MakeVector` _returnvalue_x (- _returnvalue_y (`self.Offset`)) _returnvalue_z) "World" true)
    (bind _returnvalue (`SplineComponent.GetTangentAtSplinePoint` _mainroad _index "World"))
    (`SplineComponent.SetTangentAtSplinePoint` _leftblocker _index _returnvalue "World" true)
    (bind (_returnvalue_x_2 _returnvalue_y_2 _returnvalue_z_2) (`KismetMathLibrary.BreakVector` (`SplineComponent.GetLocationAtSplinePoint` (`self.MainRoad`) _index "World")))
    (`SplineComponent.AddSplinePoint` _rightblocker (`KismetMathLibrary.MakeVector` _returnvalue_x_2 (+ _returnvalue_y_2 (`self.Offset`)) _returnvalue_z_2) "World" true)
    (`SplineComponent.SetTangentAtSplinePoint` _rightblocker _index _returnvalue "World" true)))

(fn `UserConstructionScript`
  (bind _mainroad (`self.MainRoad`))
  (bind _mainroad_2 (`self.MainRoad`))
  (bind _relativelocation (`SceneComponent.RelativeLocation` (`self.StartRoadPoint`)))
  (`SplineComponent.SetLocationAtSplinePoint` (`self.MainRoad`) 0 _relativelocation "Local" true)
  (`SplineComponent.SetLocationAtSplinePoint` (`self.CustomLeftBlockerSpline`) 0 _relativelocation "Local" true)
  (`SceneComponent.K2_SetWorldLocation` (`self.EndRoadPoint`) (`SplineComponent.GetLocationAtSplinePoint` _mainroad_2 (- (`SplineComponent.GetNumberOfSplinePoints` _mainroad_2) 1) "Local") false false)
  (for _index (range (+ (- (`SplineComponent.GetNumberOfSplinePoints` (`self.MainRoad`)) 2) 1))
    (bind _returnvalue (`AddComponent|NODE_AddSplineMeshComponent-2`))
    (`SplineMeshComponent.SetForwardAxis` _returnvalue "X" true)
    (`PrimitiveComponent.SetMaterial` _returnvalue 0 "/Game/StarterContent/Materials/M_Brick_Clay_New.M_Brick_Clay_New")
    (bind _returnvalue_2 (+ _index 1))
    (bind _returnvalue_3 (`SplineComponent.GetLocationAtSplinePoint` _mainroad _returnvalue_2 "Local"))
    (`SplineMeshComponent.SetStartAndEnd` _returnvalue (`SplineComponent.GetLocationAtSplinePoint` _mainroad _index "Local") (`SplineComponent.GetTangentAtSplinePoint` _mainroad _index "Local") _returnvalue_3 (`SplineComponent.GetTangentAtSplinePoint` _mainroad _returnvalue_2 "Local") true)
    (`SceneComponent.K2_AttachToComponent` _returnvalue (`self.MainRoad`) "None" "KeepRelative" "KeepRelative" "KeepRelative" true))
  (if (not (`self.MakeCustomBlocker`))
    (`self.SyncBlockerToMainRoad`)
    (`self.SpawnBlockerOnSpline`)
    (else
      (`self.SpawnBlockerOnCustomSplines`)))
  ; Set End Point location at the end of the spline
  (`SceneComponent.K2_SetWorldLocation` (`self.EndRoadPoint`) _returnvalue_3 false false))