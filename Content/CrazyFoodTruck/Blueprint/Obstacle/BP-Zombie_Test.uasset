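; Test zombie obstacle for the food truck game that can be crushed under the truck and reports its death to BP_HordeManager.
; Shortly after spawn it caches the horde manager and, if found, gives its mesh a random looping idle animation and random material.
; Being crushed increments the kill count, spawns a Niagara death effect and destroys the actor.
; GetDamage returns zero and IsAZoombie returns false.
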(event `self.ReceiveBeginPlay`
  (`KismetSystemLibrary.Delay` 0.3)
  (bind _returnvalue (`GameplayStatics.GetActorOfClass` "/Game/CrazyFoodTruck/BP/BP_HordeManager.BP_HordeManager_C"))
  (bind _output_get (set `self.HordeManager` _returnvalue))
  (`/Engine/EditorBlueprintResources/StandardMacros.IsValid` _output_get
    (:`Is Valid`
      (`SkeletalMeshComponent.PlayAnimation` (`self.Zombie_Running`) (`KismetArrayLibrary.Array_Random` (`self.AnimIdle`)) true)
      (`PrimitiveComponent.SetMaterial` (`self.Zombie_Running`) 0 (`KismetArrayLibrary.Array_Random` (`self.Material`))))))

(event `self.CrushUnderTruckBlueprint`
  (params (DamageAmount :type Integer))
  (`/Engine/EditorBlueprintResources/StandardMacros.IsValid` (`self.HordeManager`)
    (:`Is Valid`
      (`HordeManager.IncrementZombiesKilled` (`self.HordeManager`))
      (`NiagaraFunctionLibrary.SpawnSystemAtLocation` "/Game/CrazyFoodTruck/Visuals/VFX/NS_ZombieDeath.NS_ZombieDeath" (`self.K2_GetActorLocation`) (struct) (0.5 0.5 0.5))
      (`self.K2_DestroyActor`))))

(fn `GetDamage`
  (returns (ReturnValue :type Integer))
  (return 0))

(fn `IsAZoombie`
  (returns (ReturnValue :type Boolean))
  (return false))

(fn `UserConstructionScript`)