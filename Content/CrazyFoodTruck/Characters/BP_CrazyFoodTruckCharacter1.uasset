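; Crazy Food Truck character Blueprint that gives its static mesh a per-player outline and color.
; After a short BeginPlay delay, and on possession, it uses ArrayIndex to build parameter names and read a stencil value and color from MPC_Outline.
; The stencil drives the mesh's custom depth and the color goes to SetPlayerColor.
; Unpossession or a negative index turns custom depth off.
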(event `self.ReceiveBeginPlay`
  (bind _staticmesh (`self.StaticMesh`))
  (bind _staticmesh_2 (`self.StaticMesh`))
  (`KismetSystemLibrary.Delay` 0.2)
  (`PrimitiveComponent.SetRenderCustomDepth` _staticmesh_2 true)
  (`PrimitiveComponent.SetCustomDepthStencilWriteMask` _staticmesh_2 "ERSM_255")
  (if (>= (`self.Array Index`) 0) :!label _label
    (bind _output_get (set `self.Bit_Name` "Bit_P"))
    (bind _returnvalue (`KismetMaterialLibrary.GetScalarParameterValue` "/Game/CrazyFoodTruck/Visuals/VFX/Outline/MPC_Outline.MPC_Outline" (`KismetStringLibrary.Conv_StringToName` (`KismetStringLibrary.Concat_StrStr` _output_get (`KismetStringLibrary.Conv_IntToString` (`self.Array Index`))))))
    (`PrimitiveComponent.SetCustomDepthStencilValue` _staticmesh (`KismetMathLibrary.FTrunc` _returnvalue))
    (`PrimitiveComponent.SetRenderCustomDepth` _staticmesh true)
    (bind _output_get_2 (set `self.Bit_Name` "OutlineColor_P"))
    (bind _returnvalue_2 (`KismetMaterialLibrary.GetVectorParameterValue` "/Game/CrazyFoodTruck/Visuals/VFX/Outline/MPC_Outline.MPC_Outline" (`KismetStringLibrary.Conv_StringToName` (`KismetStringLibrary.Concat_StrStr` _output_get_2 (`KismetStringLibrary.Conv_IntToString` (`self.Array Index`))))))
    (`self.SetPlayerColor` _returnvalue_2)
    (else
      (`KismetSystemLibrary.PrintString` "Index not found" true true (struct :`R` 1.0 :`A` 1.0))
      (`PrimitiveComponent.SetRenderCustomDepth` (`self.StaticMesh`) false :!label _label_2))))

(event `self.ReceivePossessed`
  (params (NewController :type "Controller Object Reference"))
  (goto _label))

(event `self.ReceiveUnpossessed`
  (params (OldController :type "Controller Object Reference"))
  (goto _label_2))

(fn `UserConstructionScript`)