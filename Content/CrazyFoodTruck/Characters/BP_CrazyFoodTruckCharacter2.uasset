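; Player character for Crazy Food Truck that gives its robot mesh a per-player outline through custom depth stencil.
; On BeginPlay it assigns the controller ID from ArrayIndex, then after a short delay reads that index's stencil bit and color from MPC_Outline by building parameter names.
; Possession reapplies the stencil and player color, while unpossession or a negative index turns custom depth off.
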(event `self.ReceiveBeginPlay`
  (bind _array_index (`self.Array Index`))
  (bind _robot_uv_meshopti (`self.Robot_UV_meshOpti`))
  (bind _robot_uv_meshopti_2 (`self.Robot_UV_meshOpti`))
  (`GameplayStatics.SetPlayerControllerID` (`GameplayStatics.GetPlayerController` _array_index) _array_index)
  (`KismetSystemLibrary.Delay` 0.2)
  (`PrimitiveComponent.SetRenderCustomDepth` _robot_uv_meshopti true)
  (`PrimitiveComponent.SetCustomDepthStencilWriteMask` _robot_uv_meshopti "ERSM_255")
  (if (>= (`self.Array Index`) 0) :!label _label
    (bind _output_get (set `self.Bit_Name` "Bit_P"))
    (bind _returnvalue (`KismetMaterialLibrary.GetScalarParameterValue` "/Game/CrazyFoodTruck/Visuals/VFX/Outline/MPC_Outline.MPC_Outline" (`KismetStringLibrary.Conv_StringToName` (`KismetStringLibrary.Concat_StrStr` _output_get (`KismetStringLibrary.Conv_IntToString` (`self.Array Index`))))))
    (`PrimitiveComponent.SetCustomDepthStencilValue` _robot_uv_meshopti_2 (`KismetMathLibrary.FTrunc` _returnvalue))
    (`PrimitiveComponent.SetRenderCustomDepth` _robot_uv_meshopti_2 true)
    (bind _output_get_2 (set `self.Bit_Name` "OutlineColor_P"))
    (bind _returnvalue_2 (`KismetMaterialLibrary.GetVectorParameterValue` "/Game/CrazyFoodTruck/Visuals/VFX/Outline/MPC_Outline.MPC_Outline" (`KismetStringLibrary.Conv_StringToName` (`KismetStringLibrary.Concat_StrStr` _output_get_2 (`KismetStringLibrary.Conv_IntToString` (`self.Array Index`))))))
    (`self.SetPlayerColor` _returnvalue_2)
    (else
      (`KismetSystemLibrary.PrintString` "Index not found" true true (struct :`R` 1.0 :`A` 1.0))
      (`PrimitiveComponent.SetRenderCustomDepth` (`self.Robot_UV_meshOpti`) false :!label _label_2))))

(event `self.ReceivePossessed`
  (params (NewController :type "Controller Object Reference"))
  (goto _label))

(event `self.ReceiveUnpossessed`
  (params (OldController :type "Controller Object Reference"))
  (goto _label_2))

(fn `UserConstructionScript`)