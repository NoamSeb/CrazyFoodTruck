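; Player character for CrazyFoodTruck that shows a per-player custom-depth outline and works with the upgrade-phase HUD.
; BeginPlay caches the HUD, assigns the controller ID from ArrayIndex, then applies the outline after a short delay.
; Stencil value and player color come from MPC_Outline parameters named by index, reapplied on possession, with the outline hidden on unpossession.
; Pressing F triggers the HUD's logo fade and opens EndLevel after a delay.
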(event `self.ReceiveBeginPlay`
  (bind _mesh (`self.Mesh`))
  (bind _array_index (`self.Array Index`))
  (bind _mesh_2 (`self.Mesh`))
  (bind _ashud_upgrade_phase (cast `/Game/CrazyFoodTruck/UI/HUD_UpgradePhase` (`PlayerController.GetHUD` (`GameplayStatics.GetPlayerController` 0))))
  (set `self.As HUD Main Menu` _ashud_upgrade_phase)
  (`GameplayStatics.SetPlayerControllerID` (`GameplayStatics.GetPlayerController` _array_index) _array_index)
  (`KismetSystemLibrary.Delay` 0.2)
  (`PrimitiveComponent.SetRenderCustomDepth` _mesh_2 true)
  (`PrimitiveComponent.SetCustomDepthStencilWriteMask` _mesh_2 "ERSM_255")
  (if (>= (`self.Array Index`) 0) :!label _label
    (bind _output_get (set `self.Bit_Name` "Bit_P"))
    (bind _returnvalue (`KismetMaterialLibrary.GetScalarParameterValue` "/Game/CrazyFoodTruck/Visuals/VFX/Outline/MPC_Outline.MPC_Outline" (`KismetStringLibrary.Conv_StringToName` (`KismetStringLibrary.Concat_StrStr` _output_get (`KismetStringLibrary.Conv_IntToString` (`self.Array Index`))))))
    (`PrimitiveComponent.SetCustomDepthStencilValue` _mesh (`KismetMathLibrary.FTrunc` _returnvalue))
    (`PrimitiveComponent.SetRenderCustomDepth` _mesh true)
    (bind _output_get_2 (set `self.Bit_Name` "OutlineColor_P"))
    (bind _returnvalue_2 (`KismetMaterialLibrary.GetVectorParameterValue` "/Game/CrazyFoodTruck/Visuals/VFX/Outline/MPC_Outline.MPC_Outline" (`KismetStringLibrary.Conv_StringToName` (`KismetStringLibrary.Concat_StrStr` _output_get_2 (`KismetStringLibrary.Conv_IntToString` (`self.Array Index`))))))
    (`self.SetPlayerColor` _returnvalue_2)
    (else
      (`KismetSystemLibrary.PrintString` "Index not found" true true (struct :`R` 1.0 :`A` 1.0))
      (`PrimitiveComponent.SetRenderCustomDepth` (`self.Mesh`) false :!label _label_2))))

(event `self.ReceivePossessed`
  (params (NewController :type "Controller Object Reference"))
  (goto _label))

(event `self.ReceiveUnpossessed`
  (params (OldController :type "Controller Object Reference"))
  (goto _label_2))

(event `EnhancedInput|/Game/CrazyFoodTruck/Characters/Inputs/IA_Characters_Interact`
  (params (ActionValue :type Boolean) (ElapsedSeconds :type "Float (double-precision)") (TriggeredSeconds :type "Float (double-precision)") (InputAction :type "InputAction Object Reference" :default "/Game/CrazyFoodTruck/Characters/Inputs/IA_Characters_Interact.IA_Characters_Interact")))

(event `Key|F`
  (params (Key :type "Key Structure"))
  (bind _as_hud_main_menu (`self.As HUD Main Menu`))
  (:`Pressed`
    (`GameplayStatics.LoadStreamLevelBySoftObjectPtr` "/Game/CrazyFoodTruck/Levels/EndLevel.EndLevel")
    (`/Game/CrazyFoodTruck/UI/HUD_UpgradePhase.CE_CreateFade` _as_hud_main_menu)
    (`/Game/CrazyFoodTruck/UI/HUD_UpgradePhase.CE_Fade0to1WithLogo` _as_hud_main_menu)
    (`KismetSystemLibrary.Delay` 3.0)
    (`GameplayStatics.OpenLevelBySoftObjectPtr` "/Game/CrazyFoodTruck/Levels/EndLevel.EndLevel")))

(fn `UserConstructionScript`)