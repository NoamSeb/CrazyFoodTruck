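; BP_ZoneTurret is a zone Blueprint for the Crazy Food Truck turret, exposing a scalable Zone, a target point and a cursor joint.
; It holds no targeting logic: a custom event sets the Zone's world scale, and getters return that scale, the SMTarget world location and the SCCursorJoint component.
; SetPositionZone and the construction script are empty.
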(event `CE_SetScale`
  (params (`New scale` :type "Vector Structure"))
  (`SceneComponent.SetWorldScale3D` (`self.Zone`) `New scale`))

(fn `GetCursor`
  (returns (NewParam :type "SceneComponent Object Reference"))
  (return (`self.SC_CursorJoint`)))

(fn `GetScale`
  (returns (Scale :type "Vector Structure"))
  (return (`SceneComponent.K2_GetComponentScale` (`self.Zone`))))

(fn `GetTargetPosition`
  (returns (NewParam :type "Vector Structure"))
  (return (`SceneComponent.K2_GetComponentLocation` (`self.SM_Target`))))

(fn `SetPositionZone`)

(fn `UserConstructionScript`)