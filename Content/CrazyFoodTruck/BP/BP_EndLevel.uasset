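; BP_EndLevel drives the end-of-demo screen through the upgrade-phase HUD.
; On BeginPlay it casts the first player controller's HUD to HUD_UpgradePhase, then has it create a fade and the end-demo display and start a 1-to-0 fade with logo.
; After a short delay it removes the fade, with leftover debug prints around that call.
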(event `self.ReceiveBeginPlay`
  (bind _ashud_upgrade_phase (cast `/Game/CrazyFoodTruck/UI/HUD_UpgradePhase` (`PlayerController.GetHUD` (`GameplayStatics.GetPlayerController` 0))))
  (bind _output_get (set `self.As HUD Upgrade` _ashud_upgrade_phase))
  (`/Game/CrazyFoodTruck/UI/HUD_UpgradePhase.CE_CreateFade` _output_get)
  (`/Game/CrazyFoodTruck/UI/HUD_UpgradePhase.CE_CreateEndDemo` _output_get)
  (`/Game/CrazyFoodTruck/UI/HUD_UpgradePhase.CE_Fade1to0WithLogo` _output_get)
  (`KismetSystemLibrary.Delay` 1.0)
  (`KismetSystemLibrary.PrintString` "Hello")
  (`/Game/CrazyFoodTruck/UI/HUD_UpgradePhase.CE_RemoveFade` _output_get)
  (`KismetSystemLibrary.PrintString` "bfdbdw"))

(fn `UserConstructionScript`)