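; BP_ZombieIA is a zombie AI character that wanders at random and can be killed through a damage event.
; CE_Round starts on BeginPlay, resets walk speed and moves to random reachable points within a radius, repeating after a short delay on success only.
; CE_Degats subtracts from Life and destroys the actor at zero.
; OnSeePawn is empty; the sped-up player-chase logic is disconnected and never runs.
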(event `self.ReceiveBeginPlay`
  (set `self.life` 100)
  (set `self.walkSpeed` (`CharacterMovementComponent.MaxWalkSpeed` (`self.CharacterMovement`)))
  (`self.CE_Round`))

(event `CE_Degats`
  (params (degats :type Integer))
  (bind _output_get (set `self.life` (- (`self.life`) degats)))
  (if (<= _output_get 0)
    (`self.K2_DestroyActor`)))

(event `CE_Round`
  (set `CharacterMovementComponent.MaxWalkSpeed` (`self.walkSpeed`) (`self.CharacterMovement`))
  (`|AIMoveTo` self (`NavigationSystemV1.K2_GetRandomReachablePointInRadius` (`self.K2_GetActorLocation`) 1000.0 null null) null
    (:`OnSuccess`
      (`KismetSystemLibrary.Delay` 0.4)
      (`self.CE_Round`))))

(event `self.PawnSensing.OnSeePawn`
  (params (Pawn :type "Pawn Object Reference")))

(fn `UserConstructionScript`)