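; Scissor turret Blueprint for the food truck game whose arm pose is driven by an external alpha value rather than normal playback.
; On BeginPlay it puts the scissor arm mesh into single-node animation mode and assigns its animation.
; SetAnimationAlpha scales the alpha by the clip's length and scrubs the arm to that position without firing notifies, printing the computed time for debugging.
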(event `self.ReceiveBeginPlay`
  (`SkeletalMeshComponent.SetAnimationMode` (`self.ScissorArmSansAnim`) "AnimationSingleNode" true)
  (`SkeletalMeshComponent.SetAnimation` (`self.ScissorArmSansAnim`) (`self.animation`)))

(event `self.SetAnimationAlpha`
  (params (Alpha :type "Float (single-precision)"))
  (bind _returnvalue (/ (`KismetMathLibrary.Lerp` 0.0 100.0 Alpha) (/ 100.0 (`AnimationAsset.GetPlayLength` (`self.animation`)))))
  (`KismetSystemLibrary.PrintString` (`KismetStringLibrary.Conv_DoubleToString` _returnvalue))
  (`SkeletalMeshComponent.SetPosition` (`self.ScissorArmSansAnim`) _returnvalue false))

(fn `UserConstructionScript`)