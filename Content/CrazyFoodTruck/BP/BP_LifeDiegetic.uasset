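; BP_LifeDiegetic is an in-world life gauge that shows health by scaling a cylinder mesh.
; It caches the cylinder's world scale at BeginPlay as the full-life size.
; CE_UpdateLifeRender scales the base Y axis by the ratio of actual to maximum life.
; A timeline then interpolates from the current scale to that target for an animated change.
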(event `self.ReceiveBeginPlay`
  (set `self.BaseSize` (`SceneComponent.K2_GetComponentScale` (`self.M_CylinderLife`))))

(event `CE_UpdateLifeRender`
  (params (MaxLife :type Integer) (ActualLife :type Integer))
  (set `self.ActualSize` (`SceneComponent.K2_GetComponentScale` (`self.M_CylinderLife`)))
  (set `self.TargetSize` (`KismetMathLibrary.MakeVector` (.x (`self.BaseSize`)) (`KismetMathLibrary.Lerp` 0.0 (.y (`self.BaseSize`)) (/ (`KismetMathLibrary.Conv_IntToDouble` ActualLife) (`KismetMathLibrary.Conv_IntToDouble` MaxLife))) (.z (`self.BaseSize`))))
  (bind (_direction _alpha) (`Timeline|Timeline` :!via `PlayFromStart`)
    (:`Update`
      (`SceneComponent.SetWorldScale3D` (`self.M_CylinderLife`) (`KismetMathLibrary.VLerp` (`self.ActualSize`) (`self.TargetSize`) _alpha)))))

(fn `UserConstructionScript`)