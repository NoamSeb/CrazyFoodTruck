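; Zombie enemy Blueprint with a C++-triggered round start, a life widget and interface hooks for damage and truck contact.
; CallRound sends it via AIMoveTo to a first target, then repeatedly to the main target, retrying on failure.
; Non-lethal hits and truck contact briefly cut walk speed, which a Timeline eases back; crushing deals heavy damage.
; Death is broadcast before destruction, and Tick turns the widget toward the camera.
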(event `self.PawnSensing.OnSeePawn`
  (params (Pawn :type "Pawn Object Reference"))
  ; See Pawn
)

(event `self.ReceiveBeginPlay`
  ; BeginPlay
  (bind _asuw_zombie_widget (cast `/Game/CrazyFoodTruck/Widget/UW_ZombieWidget` (`WidgetComponent.GetUserWidgetObject` (`self.Widget`))))
  (set `self.UW_Widget_Zombie` _asuw_zombie_widget)
  (`/Game/CrazyFoodTruck/Widget/UW_ZombieWidget.Initialize` (`self.UW_Widget_Zombie`) (`self.life`)))

(event `CE_Round`
  ; Round
  (`/Engine/EditorBlueprintResources/StandardMacros.IsValid` (`self.CurrentActorToFollow`)
    (:`Is Valid`
      (set `CharacterMovementComponent.MaxWalkSpeed` (`self.ZombieSpeed`) (`self.CharacterMovement`))
      (`|AIMoveTo` self (0.0 0.0 0.0) (`self.CurrentActorToFollow`) 300.0
        (:`OnSuccess`
          (set `self.CurrentActorToFollow` (`self.MainActorToFollower`)))
        (:`OnFail`
          _))
      (`self.CE_Round`))))

(event `CE_KillObject`
  ; Interface
  (`self.K2_DestroyActor`))

(event `self.ReceiveDamageBlueprint`
  (params (DamageAmount :type Integer))
  ; Interface
  (bind _output_get (set `self.life` (- (`self.life`) DamageAmount)))
  (`/Game/CrazyFoodTruck/Widget/UW_ZombieWidget.UpdateLife` (`self.UW_Widget_Zombie`) _output_get)
  (`self.CE_CheckLifeCondition`))

(event `CE_CheckLifeCondition`
  ; Interface
  (if (<= (`self.life`) 0)
    (`self.BroadcastDeath` null)
    (`self.K2_DestroyActor`)
    (else
      (`self.CE_ResetVelocity`))))

(event `self.CrushUnderTruckBlueprint`
  (params (DamageAmount :type Integer))
  ; Interface
  (`IShootable.ReceiveDamageBlueprint` 100))

(event `self.InteractWithTruck`
  ; Interface
  (`self.CE_ResetVelocity`))

(event `self.CallRound`
  ; Event in C++
  (set `self.CurrentActorToFollow` (`self.FirstActorToFollower`))
  (`self.CE_Round`))

(event `CE_UpdateWidgetRotation`
  ; Update Widget Rotation
  (`SceneComponent.K2_SetWorldRotation` (`self.Widget`) (`KismetMathLibrary.FindLookAtRotation` (`SceneComponent.K2_GetComponentLocation` (`self.Widget`)) (`SceneComponent.K2_GetComponentLocation` (`PlayerCameraManager.TransformComponent` (`GameplayStatics.GetPlayerCameraManager` 0)))) false false))

(event `self.ReceiveTick`
  (params (DeltaSeconds :type "Float (single-precision)"))
  ; TICK
  (`self.CE_UpdateWidgetRotation`))

(event `CE_ResetVelocity`
  (bind _charactermovement (`self.CharacterMovement`))
  ; Zombie Hit
  (bind _output_get (set `CharacterMovementComponent.MaxWalkSpeed` (/ (`CharacterMovementComponent.MaxWalkSpeed` _charactermovement) 1.1) _charactermovement))
  (set `self.ActualRunSpeed` _output_get)
  (bind (_direction _alpha) (`Timeline|Timeline` :!via `PlayFromStart`)
    (:`Update`
      (set `CharacterMovementComponent.MaxWalkSpeed` (`KismetMathLibrary.Lerp` (`self.ActualRunSpeed`) (`self.ZombieSpeed`) _alpha) (`self.CharacterMovement`)))))

(fn `GetDamage`
  (returns (ReturnValue :type Integer))
  (return 1))

(fn `GetGroundPosition`)

(fn `IsAZoombie`
  (returns (ReturnValue :type Boolean))
  (return true))

(fn `UserConstructionScript`)