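; BP_MunitionDrawer is a drawer whose open position follows ammo updates in the Crazy Food Truck game.
; On BeginPlay it binds to OnAmmoUpdate and attaches every component in its ToChild list to the drawer mesh, keeping world transforms.
; Each update passes an open value that lerps the drawer's world location between start and end marker components, carrying the attached components along.
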(event `self.ReceiveBeginPlay`
  (add `self.OnAmmoUpdate` (delegate `OnAmmoUpdate_Event`))
  (`self.CE_SetChildList`))

(event `OnAmmoUpdate_Event` :!signature `self.OnAmmoUpdate`
  (params (CurrentOpenValue :type "Float (single-precision)"))
  (`self.CE_UpdateDrawer` CurrentOpenValue))

(event `CE_UpdateDrawer`
  (params (Float :type "Float (double-precision)"))
  (`SceneComponent.K2_SetWorldLocation` (`self.M_Drawer`) (`KismetMathLibrary.VLerp` (`SceneComponent.K2_GetComponentLocation` (`self.SC_StartPoint`)) (`SceneComponent.K2_GetComponentLocation` (`self.SC_EndPoint`)) Float) false false))

(event `CE_SetChildList`
  (for _array_element (`self.ToChild`)
    (`self.K2_AttachToComponent` _array_element (`self.M_Drawer`) "None" "KeepWorld" "KeepWorld" "KeepWorld" true)))

(fn `UserConstructionScript`)