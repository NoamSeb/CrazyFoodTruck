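; BP_EntityTest2 is a test entity in CrazyFoodTruck that shows its health through a zombie UI widget.
; On BeginPlay it casts the Widget component's user widget to UW_ZombieWidget, binds to its own OnLifeChange dispatcher and initializes the widget with current health.
; Each life change updates the widget.
; The DamageBlueprint event only prints a debug string.
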(event `self.ReceiveBeginPlay`
  (bind _asuw_zombie_widget (cast `/Game/CrazyFoodTruck/Widget/UW_ZombieWidget` (`WidgetComponent.GetUserWidgetObject` (`self.Widget`))))
  (set `self.UW_WidgetClass` _asuw_zombie_widget)
  (add `self.OnLifeChange` (delegate `OnLifeChange_Event`))
  (`/Game/CrazyFoodTruck/Widget/UW_ZombieWidget.Initialize` (`self.UW_WidgetClass`) (`self.GetHealth`)))

(event `OnLifeChange_Event` :!signature `self.OnLifeChange`
  (params (NewLife :type Integer))
  (`/Game/CrazyFoodTruck/Widget/UW_ZombieWidget.UpdateLife` (`self.UW_WidgetClass`) NewLife))

(event `self.ReceiveDamageBlueprint`
  (params (DamageAmount :type Integer))
  (`KismetSystemLibrary.PrintString` "T2"))

(fn `UserConstructionScript`)