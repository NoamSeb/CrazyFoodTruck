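; BP_AmmoSpawner is an ammo box spawner that animates each newly spawned box moving to a target point.
; On BeginPlay it binds to its OnAmmoSpawned dispatcher, which passes the spawned box to a custom animation event.
; That event stores the box's starting location, then a timeline's alpha lerps it to the TargetPoint component's world location without sweeping.
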(event `self.ReceiveBeginPlay`
  (add `self.OnAmmoSpawned` (delegate `OnAmmoSpawned_Event`)))

(event `OnAmmoSpawned_Event` :!signature `self.OnAmmoSpawned`
  (params (SpawnedAmmoBox :type "AmmoBox Object Reference"))
  (`self.CE_SpawnAnimation` SpawnedAmmoBox))

(event `CE_SpawnAnimation`
  (params (Box :type "AmmoBox Object Reference"))
  (bind _output_get (set `self.BasePosition` (`self.K2_GetActorLocation` Box)))
  (bind (_direction _y_alpha) (`Timeline|Timeline` :!via `PlayFromStart`)
    (:`Update`
      (`self.K2_SetActorLocation` Box (`KismetMathLibrary.VLerp` _output_get (`SceneComponent.K2_GetComponentLocation` (`self.TargetPoint`)) _y_alpha) false false))))

(fn `UserConstructionScript`)