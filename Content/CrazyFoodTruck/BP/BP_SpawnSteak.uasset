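; BP_SpawnSteak is a station in CrazyFoodTruck that spawns a steak for a plate entering its trigger box.
; On overlap it waits a configurable delay, then calls SpawnSteak if the plate is still under it and has no steak.
; The PlateController's movement is locked for two seconds during the spawn.
; Leaving the box clears the presence flag and restores movement.
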(event `self.ReceiveBeginPlay`
  (set `self.PlateUnderSpawn` false))

(event `self.Box.OnComponentBeginOverlap`
  (params (OverlappedComponent :type "PrimitiveComponent Object Reference") (OtherActor :type "Actor Object Reference") (OtherComp :type "PrimitiveComponent Object Reference") (OtherBodyIndex :type Integer) (bFromSweep :type Boolean) (SweepResult :type "HitResult Structure (by ref)"))
  (bind _asplate_controller (cast `PlateController` OtherActor))
  (bind _output_get (set `self.PlateUnderSpawn` true))
  (`KismetSystemLibrary.Delay` (`self.DelaySpawnSteak`))
  (if (and _output_get (== (`PlateController.HasSteak` _asplate_controller) false))
    (set `PlateController.CanMove` false _asplate_controller)
    (`self.SpawnSteak`)
    (`KismetSystemLibrary.Delay` 2.0)
    (set `PlateController.CanMove` true _asplate_controller)))

(event `self.Box.OnComponentEndOverlap`
  (params (OverlappedComponent :type "PrimitiveComponent Object Reference") (OtherActor :type "Actor Object Reference") (OtherComp :type "PrimitiveComponent Object Reference") (OtherBodyIndex :type Integer))
  (set `self.PlateUnderSpawn` false)
  (set `PlateController.CanMove` true (stale `self.Box.OnComponentBeginOverlap` _asplate_controller)))

(fn `UserConstructionScript`)