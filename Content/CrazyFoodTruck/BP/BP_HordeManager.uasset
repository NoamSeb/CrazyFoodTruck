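; BP_HordeManager drives zombie horde waves, initializing the horde zombies on BeginPlay.
; It reads the DataWave table row indexed by NbrVague, then plays the DelaySpawnHorde timeline, whose length is set to zero, before spawning.
; The row supplies zombie amount, spawn zone and target point to SpawnHordeZombie.
; It then loops to the next check until NbrVague reaches the row count, with no increment in this graph.
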(event `self.ReceiveBeginPlay`
  (bind _nbrvague (`self.nbrVague`))
  (`self.InitHordeZombies`)
  (bind _outrownames (`DataTableFunctionLibrary.GetDataTableRowNames` (`self.DataWave`) :!label _label))
  (if (< _nbrvague (`KismetArrayLibrary.Array_Length` _outrownames))
    (bind _returnvalue (`|GetDataTableRow` (`self.DataWave`) (`|GetArrayItem` _outrownames _nbrvague))
      (:`then`
        (`TimelineComponent.SetTimelineLength` (`self.DelaySpawnHorde`) 0.0)
        (`Timeline|DelaySpawnHorde` :!via `PlayFromStart`
          (:`Finished`
            (bind (_zombieamount _zonespawn _targetzombiepoint) (break `WaveStructure` _returnvalue))
            (`self.SpawnHordeZombie` _zombieamount _zonespawn _targetzombiepoint)
            (goto _label)))))))

(fn `UserConstructionScript`)