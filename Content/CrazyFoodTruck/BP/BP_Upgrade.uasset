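; BP_Upgrade sequences Crazy Food Truck's upgrade phase, from the truck's arrival to its departure for the route.
; BeginPlay initializes each character's upgrade input, sets the Amelioration phase, then slides the truck to the middle with a timeline and enables HUD and camera.
; CE_AfterUpgrade chains timelines that swing the camera's spring arm yaw and drive the truck away as the HUD fades out, then opens TestGame in Route phase.
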(event `CE_AfterUpgrade`
  (set `/Game/CrazyFoodTruck/Camera/BP_CrazyFoodTruckCameraActor.InUpgradePhase` false (`self.Camera`))
  (`self.CE_SetCam`))

(event `self.ReceiveBeginPlay`
  (bind _camera (`self.Camera`))
  (bind _foodtruck (`self.FoodTruck`))
  (bind _foodtruck_2 (`self.FoodTruck`))
  (bind _foodtruck_3 (`self.FoodTruck`))
  (bind (_returnvalue_x _returnvalue_y) (`KismetMathLibrary.BreakVector` (`self.K2_GetActorLocation` (`self.PointDepart`))))
  (bind (_returnvalue_x_2 _returnvalue_y_2 _returnvalue_z) (`KismetMathLibrary.BreakVector` (`self.K2_GetActorLocation` _foodtruck_2)))
  (bind (_returnvalue_x_3 _returnvalue_y_3) (`KismetMathLibrary.BreakVector` (`self.K2_GetActorLocation` (`self.PointDepart`))))
  (bind (_returnvalue_x_4 _returnvalue_y_4) (`KismetMathLibrary.BreakVector` (`self.K2_GetActorLocation` (`self.PointMilieu`))))
  (bind (_returnvalue_x_5 _returnvalue_y_5 _returnvalue_z_2) (`KismetMathLibrary.BreakVector` (`self.K2_GetActorLocation` _foodtruck_3)))
  (bind (_returnvalue_x_6 _returnvalue_y_6 _returnvalue_z_3) (`KismetMathLibrary.BreakVector` (`self.K2_GetActorLocation` _foodtruck)))
  (bind _asbp_crazy_food_truck_game_mode (cast `/Game/CrazyFoodTruck/GameMode/BP_CrazyFoodTruckGameMode` (`GameplayStatics.GetGameMode`)))
  (set `self.As BP Crazy Food Truck Game Mode` _asbp_crazy_food_truck_game_mode)
  (set `/Game/CrazyFoodTruck/Camera/BP_CrazyFoodTruckCameraActor.InUpgradePhase` false (`self.Camera`))
  (`KismetSystemLibrary.Delay` 0.2)
  (bind _outactors (`GameplayStatics.GetAllActorsOfClass` "/Script/CrazyFoodTruck.CrazyFoodTruckCharacter"))
  (bind _output_get (set `self.ListCharacter` _outactors))
  (for _array_element _output_get
    (bind _returnvalue (`self.GetComponentByClass` _array_element "/Script/CrazyFoodTruck.InputAmeliorationCharacters"))
    (set `InputAmeliorationCharacters.indexPlayerController` (`CrazyFoodTruckCharacter.GetPlayerIndex` _array_element) _returnvalue)
    (`InputAmeliorationCharacters.Init` _returnvalue))
  (set `GameDataSubSystem.CurrentGamePhase` "Amelioration" (subsystem `GameDataSubSystem`))
  (set `self.AlreadyFadeOut` false)
  (bind _returnvalue_2 (`GameplayStatics.GetActorOfClass` "/Game/CrazyFoodTruck/UI/HUD_UpgradePhase.HUD_UpgradePhase_C"))
  (bind _output_get_2 (set `self.HUD` _returnvalue_2))
  (set `/Game/CrazyFoodTruck/Camera/BP_CrazyFoodTruckCameraActor.InUpgradePhase` false _camera)
  (`/Game/CrazyFoodTruck/Camera/BP_CrazyFoodTruckCameraActor.CE_Init` _camera)
  (`self.K2_SetActorLocation` _foodtruck (`KismetMathLibrary.MakeVector` _returnvalue_x _returnvalue_y _returnvalue_z_3) false true)
  (`KismetSystemLibrary.Delay` 0.4)
  (bind (_direction _gotomiddle) (`Timeline|TruckToMiddle` :!via `PlayFromStart`)
    (:`Update`
      (`self.K2_SetActorLocation` _foodtruck_2 (`KismetMathLibrary.MakeVector` (`KismetMathLibrary.Lerp` _returnvalue_x_3 _returnvalue_x_4 _gotomiddle) (`KismetMathLibrary.Lerp` _returnvalue_y_3 _returnvalue_y_4 _gotomiddle) _returnvalue_z) false false))
    (:`Finished`
      (`self.K2_SetActorLocation` _foodtruck_3 (`KismetMathLibrary.MakeVector` _returnvalue_x_4 _returnvalue_y_4 _returnvalue_z_2) false false)
      (`/Game/CrazyFoodTruck/UI/HUD_UpgradePhase.CE_SetCamp` (`self.HUD`) (`self.ListCharacter`))
      (set `/Game/CrazyFoodTruck/Camera/BP_CrazyFoodTruckCameraActor.InUpgradePhase` true (`self.Camera`)))))

(event `CE_SetCam`
  (bind _springarm (`CrazyFoodTruckCameraActor.SpringArm` (`self.Camera`)))
  (bind (_returnvalue_roll _returnvalue_pitch _returnvalue_yaw) (`KismetMathLibrary.BreakRotator` (`SceneComponent.K2_GetComponentRotation` _springarm)))
  (set `self.StartRotation` _returnvalue_yaw)
  (bind (_direction _float) (`Timeline|SetCam` :!via `PlayFromStart`)
    (:`Update`
      (`SceneComponent.K2_SetWorldRotation` _springarm (`KismetMathLibrary.MakeRotator` _returnvalue_roll _returnvalue_pitch (`KismetMathLibrary.Lerp` (`self.StartRotation`) -270.0 _float)) false false))
    (:`Finished`
      (`SceneComponent.K2_SetWorldRotation` _springarm (`KismetMathLibrary.MakeRotator` _returnvalue_roll _returnvalue_pitch _returnvalue_yaw) false false)
      (set `/Game/CrazyFoodTruck/Camera/BP_CrazyFoodTruckCameraActor.InUpgradePhase` false (`self.Camera`))
      (`self.CE_TruckToEnd`))))

(event `CE_TruckToEnd`
  (bind _foodtruck (`self.FoodTruck`))
  (bind _foodtruck_2 (`self.FoodTruck`))
  (bind (_returnvalue_x _returnvalue_y) (`KismetMathLibrary.BreakVector` (`self.K2_GetActorLocation` (`self.PointArriver`))))
  (bind (_returnvalue_x_2 _returnvalue_y_2 _returnvalue_z) (`KismetMathLibrary.BreakVector` (`self.K2_GetActorLocation` _foodtruck_2)))
  (bind (_returnvalue_x_3 _returnvalue_y_3) (`KismetMathLibrary.BreakVector` (`self.K2_GetActorLocation` (`self.PointMilieu`))))
  (bind (_returnvalue_x_4 _returnvalue_y_4 _returnvalue_z_2) (`KismetMathLibrary.BreakVector` (`self.K2_GetActorLocation` _foodtruck)))
  (bind (_direction _float) (`Timeline|TruckToEnd` :!via `PlayFromStart`)
    (:`Update`
      (`self.K2_SetActorLocation` _foodtruck_2 (`KismetMathLibrary.MakeVector` (`KismetMathLibrary.Lerp` _returnvalue_x_3 _returnvalue_x _float) (`KismetMathLibrary.Lerp` _returnvalue_y_3 _returnvalue_y _float) _returnvalue_z) false false)
      (if (<= _float 0.1)
        (if (not (`self.AlreadyFadeOut`))
          (set `self.AlreadyFadeOut` true)
          (`/Game/CrazyFoodTruck/UI/HUD_UpgradePhase.CE_FadeOut` (`self.HUD`)))))
    (:`Finished`
      (`self.K2_SetActorLocation` _foodtruck (`KismetMathLibrary.MakeVector` _returnvalue_x _returnvalue_y _returnvalue_z_2) false false)
      (set `GameDataSubSystem.CurrentGamePhase` "Route" (subsystem `GameDataSubSystem`))
      (`GameplayStatics.OpenLevelBySoftObjectPtr` "/Game/CrazyFoodTruck/Levels/TestGame.TestGame"))))

(fn `UserConstructionScript`)