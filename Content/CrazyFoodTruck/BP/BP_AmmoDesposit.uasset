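; Ammo deposit Blueprint that animates a deposited ammo box moving into the deposit point.
; On BeginPlay it binds to the OnAmmoDeposited event, which passes the spawned box to the deposit animation.
; The box snaps to BaseDepositPoint, a Timeline lerps it from that cached position to TargetDepositPoint's current location, and it is destroyed when the Timeline finishes.
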(event `self.ReceiveBeginPlay`
  (add `self.OnAmmoDeposited` (delegate `OnAmmoDeposited_Event`)))

(event `OnAmmoDeposited_Event` :!signature `self.OnAmmoDeposited`
  (params (SpawnedAmmoBox :type "AmmoBox Object Reference"))
  (`self.CE_DepositAnim` SpawnedAmmoBox))

(event `CE_DepositAnim`
  (params (Box :type "AmmoBox Object Reference"))
  (bind _basedepositpoint (`self.BaseDepositPoint`))
  (`self.K2_SetActorLocation` Box (`SceneComponent.K2_GetComponentLocation` _basedepositpoint) false false)
  (bind _output_get (set `self.BasePosition` (`SceneComponent.K2_GetComponentLocation` _basedepositpoint)))
  (bind (_direction _y_alpha) (`Timeline|Timeline` :!via `PlayFromStart`)
    (:`Update`
      (`/Engine/EditorBlueprintResources/StandardMacros.IsValid` Box
        (:`Is Valid`
          (`self.K2_SetActorLocation` Box (`KismetMathLibrary.VLerp` _output_get (`SceneComponent.K2_GetComponentLocation` (`self.TargetDepositPoint`)) _y_alpha) false false))))
    (:`Finished`
      (`/Engine/EditorBlueprintResources/StandardMacros.IsValid` Box
        (:`Is Valid`
          (`self.K2_DestroyActor` Box))))))

(fn `UserConstructionScript`)