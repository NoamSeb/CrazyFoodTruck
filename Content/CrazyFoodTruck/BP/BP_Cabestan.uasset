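; BP_Cabestan is the capstan Blueprint in Crazy Food Truck, handling the looping turret-movement sound as it is pushed.
; OnCabestanPushed spawns the 2D loop and fades it in, using the IsPlayingSound flag to avoid stacking sounds on repeated calls.
; OnCabestanStopped clears the flag and fades out the stored audio component if it is still valid.
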(event `self.OnCabestanPushed`
  (if (not (`self._isPlayingSound`))
    (set `self._isPlayingSound` true)
    (bind _returnvalue (`GameplayStatics.SpawnSound2D` "/Game/CrazyFoodTruck/Sounds/SFX/SFX_Tourelle/SFX_Tourelle_Move/SFX_Tourelle_Move_Loop.SFX_Tourelle_Move_Loop" 1.0 1.0 0.0 null))
    (bind _output_get (set `self._ActualSound` _returnvalue))
    (`AudioComponent.FadeIn` _output_get 0.3 1.0 0.0 "Linear")))

(event `self.OnCabestanStopped`
  (bind __actualsound (`self._ActualSound`))
  (set `self._isPlayingSound` false)
  (`/Engine/EditorBlueprintResources/StandardMacros.IsValid` __actualsound
    (:`Is Valid`
      (`AudioComponent.FadeOut` __actualsound 0.5 0.0 "Linear"))))

(fn `UserConstructionScript`)