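; BP_Plateau is a kitchen actor, by its name and folder a tray, that travels along a referenced spline.
; A timeline, rate-scaled by TimeInSeconds, lerps distance over the spline's length and sets world location and rotation each update, printing the alpha.
; Events start, stop and reverse the movement.
; A percent-based stepping teleport is left unconnected.
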(event `CE_Move`
  (bind _spline (`/Game/CrazyFoodTruck/Cuisine/BP_SplinePlateau.Spline` (`self.Spline`)))
  (`TimelineComponent.SetPlayRate` (`self.T_Time`) (/ 1.0 (`self.TimeInSeconds`)))
  (bind (_direction _newtrack_0) (`Timeline|T_Time` :!label _label)
    (:`Update`
      (`KismetSystemLibrary.PrintString` (`KismetStringLibrary.Conv_DoubleToString` _newtrack_0))
      (bind _returnvalue (`KismetMathLibrary.Lerp` 0.0 (`SplineComponent.GetSplineLength` _spline) _newtrack_0))
      (`self.K2_SetActorLocationAndRotation` (`SplineComponent.GetLocationAtDistanceAlongSpline` _spline _returnvalue "World") (`SplineComponent.GetRotationAtDistanceAlongSpline` _spline _returnvalue "World")))))

(event `self.StopMovePlateau`
  (goto _label :!via `Stop`))

(event `self.ReverseMovePlateau`
  (goto _label :!via `Reverse`))

(event `self.ReceiveBeginPlay`)

(event `self.MovePlateau`
  (`self.CE_Move`))

(fn `UserConstructionScript`)