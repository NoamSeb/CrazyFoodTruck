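; Game mode for Crazy Food Truck that spawns extra local players for local multiplayer when play begins.
; BeginPlay loops over CreatePlayer with an automatic controller ID, giving each new player its own PlayerController.
; The remaining nodes are unconnected experiments with explicit controller IDs, input-device queries and a debug print of the local player count.
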(event `self.ReceiveBeginPlay`
  (for _ (range 5)
    (`GameplayStatics.CreatePlayer` -1)))

(fn `UserConstructionScript`)